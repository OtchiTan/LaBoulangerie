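; BP_Charater is a player Blueprint with an InventoryComponent, currently wired with hardcoded test logic for the inventory.
; On BeginPlay it constructs an LBItem named "Nisan" and appends it directly to the component's Items array, with a quantity above its own StackMax.
; Pressing Tab prints the name of the first item in that array, with no check for an empty inventory.
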(event EventBeginPlay
  (bind _returnvalue (Game|ConstructObjectfromClass "/Script/LaBoulangerie.LBItem"))
  (Variables|/Script/LaBoulangerie.LBItem|SetQuantity _returnvalue 5)
  (Variables|/Script/LaBoulangerie.LBItem|SetItemData _returnvalue (Utilities|Struct|MakeLBItemData "Nisan" 3 "/Engine/EditorResources/BadBlueprintSprite.BadBlueprintSprite"))
  (Utilities|Array|Add (Variables|/Script/LaBoulangerie.LBInventoryComponent|GetItems (Variables|Default|GetInventoryComponent)) _returnvalue))

(event Collision|EventActorBeginOverlap
  (params (OtherActor :type Actor%20Object%20Reference)))

(event EventTick
  (params (DeltaSeconds :type Float%20%28single-precision%29)))

(event Input|KeyboardEvents|Tab
  (params (Key :type Key%20Structure :default "None"))
  (:Pressed
    (Development|PrintString (Utilities|String|ToString(Name) (.Nom (Utilities|Struct|BreakLBItemData (Variables|/Script/LaBoulangerie.LBItem|GetItemData (Utilities|Array|Get(acopy) (Variables|/Script/LaBoulangerie.LBInventoryComponent|GetItems (Variables|Default|GetInventoryComponent))))))))))

(fn ConstructionScript)